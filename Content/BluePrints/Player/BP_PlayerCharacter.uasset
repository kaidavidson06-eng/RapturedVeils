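; First-person player character with movement, sprint, pause, and switchable sawn-off shotgun and rifle.
; A weapon state enum drives mesh visibility, anim class and ammo logic, with camera hitscans damaging Enemy actors.
; Timelines handle aim zoom and sensitivity, delayed health regeneration with invulnerability frames, and kill dialogue cooldown, while lethal damage opens the death screen level.
; Tick runs randomized ambient combat sounds and on-screen debug readouts.
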(event Custom|SetPlayerState
  (params (NewState :type E_PlayerStates%20Enum :default "NewEnumerator0"))
  (bind _skeletalmesh (Variables|Default|GetSkeletalMesh))
  (bind _sm_winchester (Variables|Default|GetSM_Winchester))
  (bind _sk_shotty1 (Variables|Default|GetSK_Shotty1))
  ;[0.15 0.15 0.15 0.5] State Change
  (bind _output_get (Variables|Default|SetCurrentPlayerState NewState))
  (switch Utilities|FlowControl|Switch|SwitchonE_PlayerStates _output_get
    (:NewEnumerator1
      (Development|SetHiddeninGame _sk_shotty1 true false)
      (Development|SetHiddeninGame _sm_winchester true false)
      (Components|SkeletalMesh|SetAnimInstanceClass _skeletalmesh "/Game/BluePrints/Player/MeshesAnim/ABP_DefaultAnimset.ABP_DefaultAnimset_C"))
    (:NewEnumerator2
      (Development|SetHiddeninGame _sk_shotty1 false false)
      (Development|SetHiddeninGame _sm_winchester true false)
      (Components|SkeletalMesh|SetAnimInstanceClass _skeletalmesh "/Game/BluePrints/Player/MeshesAnim/ABP_ShottyBody.ABP_ShottyBody_C"))
    (:NewEnumerator3
      (Development|SetHiddeninGame _sk_shotty1 true false)
      (Development|SetHiddeninGame _sm_winchester false false)
      (Components|SkeletalMesh|SetAnimInstanceClass _skeletalmesh "/Game/BluePrints/Player/MeshesAnim/ABP_RifleBody.ABP_RifleBody_C"))))

(event Custom|UpdateReloadBool
  (params (Value :type Boolean))
  (Variables|Default|SetIsReloading Value)
  (switch Utilities|FlowControl|Switch|SwitchonE_PlayerStates (Variables|Default|GetCurrentPlayerState)
    (:NewEnumerator2
      (|SawnOffAmmoLogic))
    (:NewEnumerator3
      (|RifleAmmoLogic))))

(event Custom|UpdateFiredBool
  (params (Value :type Boolean))
  (Utilities|FlowControl|Delay 0.1)
  (Variables|Default|SetFiredShot Value))

(event Custom|PlayerTakeDamage
  (params (DamageRecieved :type Float%20%28double-precision%29))
  (if (not (Variables|Default|GetIframe))
    (Audio|PlaySound2D "/Game/Audio/Player/Damage/SC_RD_Punch.SC_RD_Punch" 2.0 1.0 0.0 0 0)
    (CallFunction|StopRegen)
    (bind _output_get (Variables|Default|SetHealth (- (Variables|Default|GetHealth) DamageRecieved)))
    (Development|PrintString (Utilities|String|Append "Player Recieved Damage: " (Utilities|String|ToString(Float) DamageRecieved)) true false "(R=0.045611,G=0.000000,B=1.000000,A=1.000000)" 5.0)
    (if (<= _output_get 0.0)
      ;[0.15 0.15 0.15 0.5] player Fucking Dies "FUCK"
      (CallFunction|DeathEffect)
      (else
        ;[0.15 0.15 0.15 0.5] Player Doesnt Die
        (Timeline|PlayerRecentlyHit PlayFromStart
          (:Finished
            (bind _output_get_2 (Variables|Default|SetHealthToRegenFrom (Variables|Default|GetHealth)))
            (bind _health_alpha (Timeline|Regenerate%20Health PlayFromStart)
              (:Update
                (Variables|Default|SetHealth (Math|Float|Lerp _output_get_2 (Variables|Default|GetMaxHealth) _health_alpha))
                (Timeline|IFrames Play
                  (:Update
                    (Variables|Default|SetIframe true))
                  (:Finished
                    (Variables|Default|SetIframe false)))))))))))

(event Custom|StopRegen
  ;[0.15 0.15 0.15 0.5] Player Doesnt Die
  (bind _health_alpha (Timeline|Regenerate%20Health Stop)
    (:Update
      (Variables|Default|SetHealth (Math|Float|Lerp (stale Custom|PlayerTakeDamage _output_get_2) (Variables|Default|GetMaxHealth) _health_alpha))
      (Timeline|IFrames Play
        (:Update
          (Variables|Default|SetIframe true))
        (:Finished
          (Variables|Default|SetIframe false))))))

(event Custom|PlayFootstep
  (if (not (AI|Components|NavMovement|IsFalling (Variables|Character|GetCharacterMovement)))
    (if (== (Variables|/Script/Engine.CharacterMovementComponent|GetMaxWalkSpeed (Variables|Character|GetCharacterMovement)) (Variables|Default|GetRunSpeed))
      (Audio|PlaySound2D "/Game/Audio/Footsteps/SC_Run.SC_Run" 1.0 1.0 0.0 0 0)
      (else
        (Audio|PlaySound2D "/Game/Audio/Footsteps/SC_Walk.SC_Walk" 1.0 1.0 0.0 0 0)))))

(event Custom|ShotFiredOverride)

(event Custom|CheckForEmptyMag
  (switch Utilities|FlowControl|Switch|SwitchonE_PlayerStates (Variables|Default|GetCurrentPlayerState)
    (:NewEnumerator2
      (if (<= (Variables|Default|GetShotgunChamberCurrent) 0)
        (Variables|Default|SetFiredShot false :!label _label)
        (if (Variables|Default|GetFiredShot)
          (Utilities|FlowControl|Delay 0.2))
        (switch Utilities|FlowControl|Switch|SwitchonE_PlayerStates (Variables|Default|GetCurrentPlayerState)
          (:NewEnumerator2
            (|SawnOffReloadLogic))
          (:NewEnumerator3
            (|RifleReloadLogic_2)))))
    (:NewEnumerator3
      (if (<= (Variables|Default|GetRifleMagCurrent) 0)
        (goto _label)))))

(event Custom|KillDialogue
  (if (not (Variables|Default|GetSpeakingSideDialogue))
    (Variables|Default|SetSpeakingSideDialogue true)
    (Audio|PlaySound2D "/Game/Audio/Dialogue/KillDialogue/SC_KillDialogue.SC_KillDialogue" 1.0 1.0 0.0 0 0)
    (Timeline|KillDialogueRefresh PlayFromStart
      (:Finished
        (Variables|Default|SetSpeakingSideDialogue false)))))

(event Input|EnhancedActionEvents|EnhancedInputActionIA_Crouch
  (params (ActionValue :type Boolean) (ElapsedSeconds :type Float%20%28double-precision%29) (TriggeredSeconds :type Float%20%28double-precision%29) (InputAction :type Input%20Action%20Object%20Reference :default "/Game/BluePrints/Player/Inputs/IA_Crouch.IA_Crouch")))

(event Input|EnhancedActionEvents|EnhancedInputActionIA_WASD
  (params (ActionValue :type Vector%202D%20Structure) (ElapsedSeconds :type Float%20%28double-precision%29) (TriggeredSeconds :type Float%20%28double-precision%29) (InputAction :type Input%20Action%20Object%20Reference :default "/Game/BluePrints/Player/Inputs/IA_WASD.IA_WASD"))
  (Pawn|Input|AddMovementInput (+ (* (.y ActionValue) (Transformation|GetActorRightVector)) (* (.x ActionValue) (Transformation|GetActorForwardVector))) 1.0 false))

(event Input|EnhancedActionEvents|EnhancedInputActionIA_Pause
  (params (ActionValue :type Boolean) (ElapsedSeconds :type Float%20%28double-precision%29) (TriggeredSeconds :type Float%20%28double-precision%29) (InputAction :type Input%20Action%20Object%20Reference :default "/Game/BluePrints/Player/Inputs/IA_Pause.IA_Pause"))
  (Game|SetGamePaused true)
  (bind _returnvalue (UserInterface|CreateWidget "/Game/UI/Pause_Menu/PauseMenuWB.PauseMenuWB_C"))
  (Variables|/Script/Engine.PlayerController|SetbShowMouseCursor (Game|GetPlayerController 0) true)
  (Input|SetInputModeUIOnly (Game|GetPlayerController 0) 0 "DoNotLock" false)
  (UserInterface|Viewport|AddtoViewport _returnvalue 0))

(event Input|EnhancedActionEvents|EnhancedInputActionIA_Look
  (params (ActionValue :type Vector%202D%20Structure) (ElapsedSeconds :type Float%20%28double-precision%29) (TriggeredSeconds :type Float%20%28double-precision%29) (InputAction :type Input%20Action%20Object%20Reference :default "/Game/FirstPerson/Input/Actions/IA_Look.IA_Look"))
  (bind _mousesensitivitymultiplier (Variables|Default|GetMouseSensitivityMultiplier))
  (Pawn|Input|AddControllerYawInput (* (.x ActionValue) _mousesensitivitymultiplier))
  (Pawn|Input|AddControllerPitchInput (* (* (.y ActionValue) _mousesensitivitymultiplier) -1.0)))

(event Input|EnhancedActionEvents|EnhancedInputActionIA_Sprint
  (params (ActionValue :type Boolean) (ElapsedSeconds :type Float%20%28double-precision%29) (TriggeredSeconds :type Float%20%28double-precision%29) (InputAction :type Input%20Action%20Object%20Reference :default "/Game/BluePrints/Player/Inputs/IA_Sprint.IA_Sprint"))
  (bind _charactermovement (Variables|Character|GetCharacterMovement))
  (:Started
    (Variables|/Script/Engine.CharacterMovementComponent|SetMaxWalkSpeed _charactermovement (Variables|Default|GetRunSpeed)))
  (:Completed
    (Variables|/Script/Engine.CharacterMovementComponent|SetMaxWalkSpeed _charactermovement (Variables|Default|GetWalkSpeed))))

(event Input|EnhancedActionEvents|EnhancedInputActionIA_Jump
  (params (ActionValue :type Boolean) (ElapsedSeconds :type Float%20%28double-precision%29) (TriggeredSeconds :type Float%20%28double-precision%29) (InputAction :type Input%20Action%20Object%20Reference :default "/Game/FirstPerson/Input/Actions/IA_Jump.IA_Jump")))

(event Input|EnhancedActionEvents|EnhancedInputActionIA_Aim
  (params (ActionValue :type Boolean) (ElapsedSeconds :type Float%20%28double-precision%29) (TriggeredSeconds :type Float%20%28double-precision%29) (InputAction :type Input%20Action%20Object%20Reference :default "/Game/BluePrints/Player/Inputs/IA_Aim.IA_Aim"))
  (:Triggered
    (if (Variables|Default|GetIsReloading)
      (Variables|Default|SetIsAiming false :!label _label)
      (bind _fov_alpha (Timeline|ChangeFOV Reverse)
        (:Update
          (Camera|SetFieldOfView (Variables|Default|GetPlayerCamera) (Math|Float|Lerp 9e+01 6e+01 _fov_alpha))
          (Variables|Default|SetMouseSensitivityMultiplier (Math|Float|Lerp 1.0 0.35 _fov_alpha))))
      (else
        (Variables|Default|SetIsAiming true)
        (Timeline|ChangeFOV Play))))
  (:Started
    (Audio|PlaySound2D "/Game/Audio/ClothFoley/SC_ClothFoley.SC_ClothFoley" 0.3 1.0 0.0 0 0))
  (:Completed
    (Audio|PlaySound2D "/Game/Audio/ClothFoley/SC_ClothFoley.SC_ClothFoley" 0.1 1.0 0.0 0 0)
    (goto _label)))

(event Input|EnhancedActionEvents|EnhancedInputActionIA_EquipShotty
  (params (ActionValue :type Boolean) (ElapsedSeconds :type Float%20%28double-precision%29) (TriggeredSeconds :type Float%20%28double-precision%29) (InputAction :type Input%20Action%20Object%20Reference :default "/Game/BluePrints/Player/Inputs/IA_EquipShotty.IA_EquipShotty"))
  (CallFunction|SetPlayerState "NewEnumerator2")
  (Variables|Default|SetIsReloading false))

(event Input|EnhancedActionEvents|EnhancedInputActionIA_Fire
  (params (ActionValue :type Boolean) (ElapsedSeconds :type Float%20%28double-precision%29) (TriggeredSeconds :type Float%20%28double-precision%29) (InputAction :type Input%20Action%20Object%20Reference :default "/Game/BluePrints/Player/Inputs/IA_Fire.IA_Fire"))
  (:Started
    (switch Utilities|FlowControl|Switch|SwitchonE_PlayerStates (Variables|Default|GetCurrentPlayerState)
      (:NewEnumerator2
        (if (<= (Variables|Default|GetShotgunChamberCurrent) 0)
          (Variables|Default|SetIsAiming false)
          (else
            (Variables|Default|SetIsAiming true :!label _label)
            (switch Utilities|FlowControl|Switch|SwitchonE_PlayerStates (Variables|Default|GetCurrentPlayerState)
              (:NewEnumerator2
                (if (not (Variables|Default|GetIsReloading))
                  (if (Variables|Default|GetIsAiming)
                    (if (!= (Variables|Default|GetFiredShot) true)
                      (if (> (Variables|Default|GetShotgunChamberCurrent) 0)
                        (Variables|Default|SetShotgunChamberCurrent (- (Variables|Default|GetShotgunChamberCurrent) 1))
                        (Variables|Default|SetFiredShot true)
                        (Audio|PlaySoundatLocation "/Game/Audio/Shotgun/Shoot/SC_ShotgunShot.SC_ShotgunShot" "0, 0, 0" "0, 0, 0" 1.0 1.0 0.0 0 0 0 0) ; Play firing sound
                        (Niagara|SpawnSystemAttached "/Game/ART/Niagra/NS_BurstBullet.NS_BurstBullet" (Variables|Default|GetSK_Shotty1) "Chamber" "0.000000,-0.071293,0.303168" "90.000000,180.000000,180.000000" "KeepRelativeOffset" false)
                        (bind (_hitresult _hitsomething) (CallFunction|HitScanfromCamera 1e+04))
                        (if _hitsomething
                          (bind _asenemy (Utilities|Casting|CastToEnemy (.hitactor _hitresult)))
                          (Game|Damage|ApplyDamage _asenemy 1.0 0 0)))))))
              (:NewEnumerator3
                (if (not (Variables|Default|GetIsReloading))
                  (if (Variables|Default|GetIsAiming)
                    (if (!= (Variables|Default|GetFiredShot) true)
                      (if (> (Variables|Default|GetRifleMagCurrent) 0)
                        (Variables|Default|SetRifleMagCurrent (- (Variables|Default|GetRifleMagCurrent) 1))
                        (Variables|Default|SetFiredShot true)
                        (Audio|PlaySoundatLocation "/Game/Audio/RifleSounds/RifleShots/SC_RifleShot.SC_RifleShot" "0, 0, 0" "0, 0, 0" 1.0 1.0 0.0 0 0 0 0) ; Play firing sound
                        (Niagara|SpawnSystemAttached "/Game/ART/Niagra/NS_BurstBullet.NS_BurstBullet" (Variables|Default|GetSM_Winchester) "None" "0.343509,68.394778,7.298999" "-2.306079,92.469133,-3.234523" "KeepRelativeOffset" false)
                        (bind (_hitresult_2 _hitsomething_2) (CallFunction|HitScanfromCamera 1e+04))
                        (if _hitsomething_2
                          (bind _asenemy_2 (Utilities|Casting|CastToEnemy (.hitactor _hitresult_2)))
                          (Game|Damage|ApplyDamage _asenemy_2 1.0 0 0)))))))))))
      (:NewEnumerator3
        (if (<= (Variables|Default|GetRifleMagCurrent) 0)
          (Variables|Default|SetIsAiming false)
          (else
            (goto _label))))))
  (:Completed
    (Variables|Default|SetIsAiming false)))

(event Input|EnhancedActionEvents|EnhancedInputActionIA_Reload
  (params (ActionValue :type Boolean) (ElapsedSeconds :type Float%20%28double-precision%29) (TriggeredSeconds :type Float%20%28double-precision%29) (InputAction :type Input%20Action%20Object%20Reference :default "/Game/BluePrints/Player/Inputs/IA_Reload.IA_Reload"))
  (:Started
    (if (Variables|Default|GetFiredShot)
      (Utilities|FlowControl|Delay 0.2))
    (switch Utilities|FlowControl|Switch|SwitchonE_PlayerStates (Variables|Default|GetCurrentPlayerState)
      (:NewEnumerator2
        (|SawnOffReloadLogic))
      (:NewEnumerator3
        (|RifleReloadLogic_2)))))

(event Input|EnhancedActionEvents|EnhancedInputActionIA_EquipRifle
  (params (ActionValue :type Boolean) (ElapsedSeconds :type Float%20%28double-precision%29) (TriggeredSeconds :type Float%20%28double-precision%29) (InputAction :type Input%20Action%20Object%20Reference :default "/Game/BluePrints/Player/Inputs/IA_EquipRifle.IA_EquipRifle"))
  (CallFunction|SetPlayerState "NewEnumerator3")
  (Variables|Default|SetIsReloading false))

(event EventBeginPlay
  (Input|AddMappingContext (PlayerController|LocalPlayerSubsystems|GetEnhancedInputLocalPlayerSubsystem (Game|GetPlayerController 0)) "/Game/BluePrints/Player/Inputs/IMC_PlayerController.IMC_PlayerController" 0 "(bIgnoreAllPressedKeysUntilRelease=True,bForceImmediately=False,bNotifyUserSettings=False)")
  (CallFunction|SetPlayerState "NewEnumerator2")
  (bind _returnvalue (UserInterface|CreateWidget "/Game/WraithWaves/UI/PlayerHealth.PlayerHealth_C" (Game|GetPlayerController 0)))
  (UserInterface|Viewport|AddtoViewport _returnvalue 0))

(event EventTick
  (params (DeltaSeconds :type Float%20%28single-precision%29))
  (bind _source_out (CallFunction|PlayAmbient 2.0 1.0 "/Game/Audio/Ambient/DistantGunshots/SC_DistantGunshot.SC_DistantGunshot" (Variables|Default|GetAmbientBulletCurrent)))
  (Variables|Default|SetAmbientBulletCurrent _source_out)
  (bind _source_out_2 (CallFunction|PlayAmbient 1e+01 5.0 "/Game/Audio/Ambient/Rumble/SC_Rumble.SC_Rumble" (Variables|Default|GetAmbientExplosionCurrent)))
  (Variables|Default|SetAmbientExplosionCurrent _source_out_2)
  ;[0.15 0.15 0.15 0.5] Debugging
  (Development|PrintString (Utilities|String|Append "PlayerHealth: " (Utilities|String|ToString(Float) (Variables|Default|GetHealth))) true false "(R=0.000000,G=0.660000,B=1.000000,A=1.000000)" 0.0)
  (Development|PrintString (Utilities|String|Append "IsReloading: " (Utilities|String|ToString(Boolean) (Variables|Default|GetIsReloading))) true false "(R=1.000000,G=0.000000,B=0.075154,A=1.000000)" 0.0)
  (Development|PrintString (Utilities|String|Append "IsShooting: " (Utilities|String|ToString(Boolean) (Variables|Default|GetFiredShot))) true false "(R=1.000000,G=0.000000,B=0.075154,A=1.000000)" 0.0)
  (Development|PrintString (Utilities|String|Append "IsAiming: " (Utilities|String|ToString(Boolean) (Variables|Default|GetIsAiming))) true false "(R=1.000000,G=0.000000,B=0.075154,A=1.000000)" 0.0)
  (switch Utilities|FlowControl|Switch|SwitchonE_PlayerStates (Variables|Default|GetCurrentPlayerState)
    (:NewEnumerator2
      (Development|PrintString (Utilities|String|Append "ShotgunReserves:  " (Utilities|String|ToString(Integer) (Variables|Default|GetShotgunReserves))) true false "(R=0.000000,G=1.000000,B=0.229772,A=1.000000)" 0.0)
      (Development|PrintString (Utilities|String|Append "ShotgunChamberCurrent:  " (Utilities|String|ToString(Integer) (Variables|Default|GetShotgunChamberCurrent))) true false "(R=0.000000,G=1.000000,B=0.229772,A=1.000000)" 0.0)
      (Development|PrintString (Utilities|String|Append "ShotgunChamberMax:  " (Utilities|String|ToString(Integer) (Variables|Default|GetShotgunChamberMax))) true false "(R=0.000000,G=1.000000,B=0.229772,A=1.000000)" 0.0))
    (:NewEnumerator3
      (Development|PrintString (Utilities|String|Append "RifleReserves:  " (Utilities|String|ToString(Integer) (Variables|Default|GetRifleReserves))) true false "(R=0.000000,G=1.000000,B=0.229772,A=1.000000)" 0.0)
      (Development|PrintString (Utilities|String|Append "RifleMagCurrent:  " (Utilities|String|ToString(Integer) (Variables|Default|GetRifleMagCurrent))) true false "(R=0.000000,G=1.000000,B=0.229772,A=1.000000)" 0.0)
      (Development|PrintString (Utilities|String|Append "RifleMagMax:  " (Utilities|String|ToString(Integer) (Variables|Default|GetRifleMagMax))) true false "(R=0.000000,G=1.000000,B=0.229772,A=1.000000)" 0.0))))

(event Input|KeyboardEvents|6
  (params (Key :type Key%20Structure :default "None"))
  ;[0.1892 0.00515 0] DEBUG TESTING
)

(event Input|KeyboardEvents|5
  (params (Key :type Key%20Structure :default "None"))
  ;[0.1892 0.00515 0] DEBUG TESTING
)

(event Input|KeyboardEvents|7
  (params (Key :type Key%20Structure :default "None")))

(event Input|KeyboardEvents|0
  (params (Key :type Key%20Structure :default "None")))

(fn ConstructionScript)

(fn TakeDamage
  (params (DamageAmount :type Float%20%28double-precision%29))
  (Variables|Default|SetHealth (Math|Float|Clamp(Float) (- (Variables|Default|GetHealth) DamageAmount) 0.0 (Variables|Default|GetMaxHealth)))
  (if (<= (Variables|Default|GetHealth) 0.0)
    _))

(fn DeathEffect
  (Game|OpenLevel(byName) "Death_Screen"))

(fn HitScanfromCamera
  (params (LineTraceDistance :type Float%20%28double-precision%29))
  (bind _playercamera (Variables|Default|GetPlayerCamera))
  (bind _returnvalue (Transformation|GetWorldLocation _playercamera))
  (bind (_outhit _returnvalue_2) (Collision|LineTraceByChannel _returnvalue (+ _returnvalue (* (Math|Vector|GetForwardVector _playercamera) LineTraceDistance)) "TraceTypeQuery1" false (Variables|Default|GetCollisionActors) "ForDuration" true "(R=1.000000,G=0.000000,B=0.000000,A=1.000000)" "(R=0.000000,G=1.000000,B=0.000000,A=1.000000)" 15.0))
  (return _outhit _returnvalue_2))

(fn PlayAmbient
  (params (Frequency%20Max :type Float%20%28double-precision%29) (Frequency%20Min :type Float%20%28double-precision%29) (Sound%20Asset :type Sound%20Base%20Object%20Reference) (Source%20Current :type Float%20%28double-precision%29))
  (if (> Source%20Current Frequency%20Max)
    (Audio|PlaySound2D Sound%20Asset 0.5 1.0 0.0 0 0)
    (return (Math|Random|RandomFloatinRange Frequency%20Min Frequency%20Max))
    (else
      (return (+ Source%20Current (Utilities|Time|GetWorldDeltaSeconds))))))